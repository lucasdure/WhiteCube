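; LittleGuys character Blueprint that sets up a first-person-style view: the local player sees arms and an invisible body, while others see no arms.
; The construction script slaves Arms to Mesh via master pose.
; On possession, an owning-client event waits for player control, applies the invisible material locally, then relays through server and multicast so non-local machines destroy Arms.
; Characters not meant for player control also lose their Arms.
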(event `self.ReceiveBeginPlay`
  (`parent.ReceiveBeginPlay`))

(event `self.ReceivePossessed`
  (params (NewController :type "Controller Object Reference"))
  ;[1 1 1] SetUpBodyInvisible
  (`self.PossessEventToOwningClient`))

(event `PossessEventToOwningClient`
  ;[1 1 1] SetUpBodyInvisible
  (if (`self.ShouldBePlayerControlled`)
    (`/Game/GameplayEntities/FunctionsMacros/NetworkMacros.WaitPlayerControl` self
      (:`Out`
        (`/Game/GameplayEntities/FunctionsMacros/NetworkMacros.IsLocalPlayer` self
          (:`LocalPlayer`
            (`PrimitiveComponent.SetMaterial` (`self.Mesh`) 0 "/Game/Environment/Materials/Effect/Invisible.Invisible")
            (`self.PossessEventToServer`))
          (:`NotLocalPlayer`
            (`ActorComponent.K2_DestroyComponent` (`self.Arms`) :!label _label)))))
    (else
      (goto _label))))

(event `PossessEventToServer`
  ;[1 1 1] SetUpBodyInvisible
  (`self.PossessEventToMulti`))

(event `PossessEventToMulti`
  ;[1 1 1] SetUpBodyInvisible
  (`/Game/GameplayEntities/FunctionsMacros/NetworkMacros.IsLocalPlayer` self
    (:`NotLocalPlayer`
      (goto _label))))

(fn `UserConstructionScript`
  (`parent.UserConstructionScript`)
  (`SkinnedMeshComponent.SetLeaderPoseComponent` (`self.Arms`) (`self.Mesh`) false))