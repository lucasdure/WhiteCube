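; RiftDecalCubeBP is a six-sided decal actor that displays rift textures on world cubes according to their remaining life.
; Construction creates a dynamic material per face, stored in an indexed list.
; UpdateDecalServer relays to UpdateDecalMulti, which updates the texture only on the non-local-player branch.
; UpdateDecalTexture maps life points inversely onto the cube class's texture array, or applies the supplied Invisible texture, for one face.
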(event `UpdateDecalMulti`
  (params (Index :type Integer) (CubeState :type "/Game/Environment/WorldGenerated/Cubes/VoxelCube Structure") (Invisible :type Boolean))
  ;[1 1 1] Update decal texture
  (`/Game/GameplayEntities/FunctionsMacros/NetworkMacros.IsLocalPlayer` (`self.PawnRef`)
    (:`NotLocalPlayer`
      (`self.UpdateDecalTexture` Index CubeState Invisible))))

(event `UpdateDecalServer`
  (params (Index :type Integer) (CubeState :type "/Game/Environment/WorldGenerated/Cubes/VoxelCube Structure") (Invisible :type Boolean))
  ;[1 1 1] Update decal texture
  (`self.UpdateDecalMulti` Index CubeState Invisible))

(fn `UpdateDecalTexture`
  (params (Index :type Integer) (CubeState :type "/Game/Environment/WorldGenerated/Cubes/VoxelCube Structure") (Invisible :type Boolean))
  (bind ((`LifePoint_7_2AE7D0284340A801030E65933C61E758` _lifepoint) (`CubeClass_11_44738CB64AC6387D72F57B94318970DB` _cubeclass)) (break `/Game/Environment/WorldGenerated/Cubes/VoxelCube` CubeState))
  (bind (_maxlifepoint _decalriftstextures) (defaults `Object` _cubeclass))
  (`MaterialInstanceDynamic.SetTextureParameterValue` (`|GetArrayItem` (`self.MaterialsList`) Index) "TextureDiffuse" (select `bool` Invisible :`false` (`|GetArrayItem` _decalriftstextures (`KismetMathLibrary.FFloor` (`KismetMathLibrary.MapRangeClamped` (`KismetMathLibrary.Conv_IntToDouble` _lifepoint) 0.0 (`KismetMathLibrary.Conv_IntToDouble` _maxlifepoint) (`KismetMathLibrary.Conv_IntToDouble` (`KismetArrayLibrary.Array_Length` _decalriftstextures))))) :`true` "/Game/Environment/Textures/SimpleTextures/Invisible.Invisible" :!type "Texture Object Reference")))

(fn `UserConstructionScript`
  (for _index (range 6)
    (bind _returnvalue (`DecalComponent.CreateDynamicMaterialInstance` (select `int` _index :`0` (`self.Front`) :`1` (`self.Behind`) :`2` (`self.Right`) :`3` (`self.Left`) :`4` (`self.Top`) :`5` (`self.Bot`))))
    (`KismetArrayLibrary.Array_Add` (`self.MaterialsList`) _returnvalue)))